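; Openable door actor that swings on its yaw axis when its OpenDoor OnOpen and OnClose events fire.
; A timeline plays to open and reverses to close, setting the actor's rotation from its angle curve and playing a sound at the door on an event track.
; The starting rotation is saved on BeginPlay but never used, so the yaw is absolute.
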(event `self.ReceiveBeginPlay`
  (set `self.NewVar_0` (`self.K2_GetActorRotation`)))

(event `self.OpenDoor.OnOpen`
  (bind (_direction _openangle) (`Timeline|Timeline_0` :!label _label)
    (:`Update`
      (`self.K2_SetActorRotation` (`KismetMathLibrary.ComposeRotators` (`KismetMathLibrary.MakeRotator` 0.0 0.0 _openangle) (`KismetMathLibrary.MakeRotator` 0.0))))
    (:`Sound timing`
      (`GameplayStatics.PlaySoundAtLocation` "/Game/StarterContent/Audio/Collapse01.Collapse01" (`self.K2_GetActorLocation`) (struct) 1.0 1.0 0.0 null null null))))

(event `self.OpenDoor.OnClose`
  (goto _label :!via `Reverse`))

(fn `UserConstructionScript`)